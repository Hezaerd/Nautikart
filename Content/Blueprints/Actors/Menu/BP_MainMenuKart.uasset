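; Main menu kart actor that drives itself along the spline of the BP_MenuSpline actor found in the level.
; On BeginPlay it caches that spline actor and plays a timeline with its rate set to the inverse of TimeToComplete.
; Each update maps the timeline alpha to distance along the spline and sets the kart's location and rotation from it, sampled in the spline's local space.
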(event `self.ReceiveBeginPlay`
  (bind _returnvalue (`GameplayStatics.GetActorOfClass` "/Game/Blueprints/Actors/Menu/BP_MenuSpline.BP_MenuSpline_C"))
  (set `self.SpineRef` _returnvalue)
  (`self.Move Object`))

(event `Move Object`
  (bind _spline (`/Game/Blueprints/Actors/Menu/BP_MenuSpline.Spline` (`self.SpineRef`)))
  (`TimelineComponent.SetPlayRate` (`self.Move Object T`) (/ 1.0 (`self.TimeToComplete`)))
  (bind (_direction _move_track) (`Timeline|Move Object T`)
    (:`Update`
      (bind _returnvalue (`KismetMathLibrary.Lerp` 0.0 (`SplineComponent.GetSplineLength` (`/Game/Blueprints/Actors/Menu/BP_MenuSpline.Spline` (`self.SpineRef`))) _move_track))
      (`self.K2_SetActorTransform` (`KismetMathLibrary.MakeTransform` (`SplineComponent.GetLocationAtDistanceAlongSpline` _spline _returnvalue "Local") (`SplineComponent.GetRotationAtDistanceAlongSpline` _spline _returnvalue "Local"))))))

(fn `UserConstructionScript`)