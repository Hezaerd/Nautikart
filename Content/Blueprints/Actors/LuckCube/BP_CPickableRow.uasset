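; BP_CPickableRow is a LuckCube actor that groups three pickables into a single row.
; On BeginPlay it casts the child actors of its three BPPickable components to Pickable and stores them in the Row array.
; A failed cast stops the chain before Row is assigned, and the construction script is empty.
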(event `self.ReceiveBeginPlay`
  (bind _aspickable (cast `Pickable` (`ChildActorComponent.ChildActor` (`self.BP_Pickable`))))
  (bind _aspickable_2 (cast `Pickable` (`ChildActorComponent.ChildActor` (`self.BP_Pickable1`))))
  (bind _aspickable_3 (cast `Pickable` (`ChildActorComponent.ChildActor` (`self.BP_Pickable2`))))
  (set `self.row` (`|MakeArray` _aspickable _aspickable_2 _aspickable_3)))

(fn `UserConstructionScript`)