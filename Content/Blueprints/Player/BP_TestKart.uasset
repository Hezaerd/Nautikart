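; Test player kart driven by a physics sphere, with the kart mesh snapped to the sphere each tick.
; Four downward wheel traces average the surface normal to align mesh roll and pitch, then steering input adds yaw.
; Throttle eases a clamped speed toward its target, setting sphere velocity along mesh forward plus gravity.
; OnGround is always set true after alignment, so gravity always follows the mesh's up axis.
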(event `InputAxis|accelerate`
  (params (AxisValue :type "Float (single-precision)"))
  (set `self.accelerateValue` AxisValue))

(event `InputAxis|steer`
  (params (AxisValue :type "Float (single-precision)"))
  (set `self.steerValue` AxisValue))

(event `self.ReceiveTick`
  (params (DeltaSeconds :type "Float (single-precision)"))
  (`SceneComponent.K2_SetWorldLocation` (`self.kartMesh`) (`SceneComponent.K2_GetComponentLocation` (`self.Sphere1`)) false false)
  (`self.rotateFromNormal`)
  (`self.Steer` DeltaSeconds)
  (`self.calcCurrentSpeed`)
  (`self.Move`))

(fn `calcCurrentSpeed`
  (bind _maxspeed (`self.maxSpeed`))
  (bind _returnvalue (* _maxspeed -1.0))
  (bind _step (`self.smoothStep` (`self.currSpeed`) (* (`self.maxSpeed`) (`self.accelerateValue`)) (`self.accelerateStep`)))
  (bind _output_get (set `self.currSpeed` (+ _step (`self.currSpeed`))))
  (if (> _output_get _maxspeed)
    (set `self.currSpeed` (`self.maxSpeed`))
    (elif (< _output_get _returnvalue)
      (set `self.currSpeed` _returnvalue))))

(fn `GetWheelNormal`
  (params (wheel :type "StaticMeshComponent Object Reference"))
  (returns (normal :type "Vector Structure"))
  (locals (NewLocalVar :type "HitResult Structure"))
  (bind _returnvalue (`SceneComponent.K2_GetComponentLocation` wheel))
  (bind (_outhit _returnvalue_2) (`KismetSystemLibrary.LineTraceSingle` :`Start` _returnvalue :`End` (+ _returnvalue (* (`SceneComponent.GetUpVector` wheel) -100.0)) :`TraceChannel` "TraceTypeQuery1" :`DrawDebugType` "ForOneFrame"))
  (if _returnvalue_2
    (return (`.ImpactNormal` (`GameplayStatics.BreakHitResult` _outhit)))
    (else
      (return (0.0 0.0 0.0)))))

(fn `Move`
  (bind _sphere1 (`self.Sphere1`))
  (bind _gravity (`self.gravity`))
  (bind _returnvalue (* (`SceneComponent.GetForwardVector` (`self.kartMesh`)) (`self.currSpeed`)))
  (if (`self.onGround`)
    (`PrimitiveComponent.SetPhysicsLinearVelocity` _sphere1 (+ (* (`SceneComponent.GetUpVector` (`self.kartMesh`)) _gravity) _returnvalue) false "None")
    (else
      (`PrimitiveComponent.SetPhysicsLinearVelocity` _sphere1 (+ _returnvalue (* (`KismetMathLibrary.GetUpVector` (struct)) _gravity)) false "None"))))

(fn `rotateFromNormal`
  (bind _kartmesh (`self.kartMesh`))
  (bind (_returnvalue_roll _returnvalue_pitch _returnvalue_yaw) (`KismetMathLibrary.BreakRotator` (`SceneComponent.K2_GetComponentRotation` _kartmesh)))
  (set `self.normal` (0.0 0.0 0.0))
  (bind _normal (`self.GetWheelNormal` (`self.wheel1`)))
  (bind _output_get (set `self.normal` _normal))
  (bind _normal_2 (`self.GetWheelNormal` (`self.wheel2`)))
  (bind _output_get_2 (set `self.normal` (+ _output_get _normal_2)))
  (bind _normal_3 (`self.GetWheelNormal` (`self.wheel3`)))
  (bind _output_get_3 (set `self.normal` (+ _output_get_2 _normal_3)))
  (bind _normal_4 (`self.GetWheelNormal` (`self.wheel4`)))
  (bind _output_get_4 (set `self.normal` (+ _output_get_3 _normal_4)))
  (bind _output_get_5 (set `self.normal` (/ _output_get_4 4.0)))
  (bind _returnvalue_roll_2 (`KismetMathLibrary.BreakRotator` (`KismetMathLibrary.MakeRotFromXZ` (`SceneComponent.GetForwardVector` _kartmesh) _output_get_5)))
  (bind (_returnvalue_roll_3 _returnvalue_pitch_2) (`KismetMathLibrary.BreakRotator` (`KismetMathLibrary.MakeRotFromYZ` (`SceneComponent.GetRightVector` _kartmesh) _output_get_5)))
  (`SceneComponent.K2_SetWorldRotation` _kartmesh (`KismetMathLibrary.MakeRotator` _returnvalue_roll_2 _returnvalue_pitch_2 _returnvalue_yaw) false false)
  (set `self.onGround` true))

(fn `smoothStep`
  (params (float1 :type "Float (double-precision)") (float2 :type "Float (double-precision)") (stepAmount :type "Float (double-precision)"))
  (returns (step :type "Float (double-precision)"))
  (bind _returnvalue (`KismetMathLibrary.FClamp` stepAmount))
  (if (> float1 float2)
    (return (* (`KismetMathLibrary.Abs` (* (- float1 float2) _returnvalue)) -1.0))
    (else
      (return (`KismetMathLibrary.Abs` (* (- float2 float1) _returnvalue))))))

(fn `Steer`
  (params (delta :type "Float (double-precision)"))
  (bind (_returnvalue_roll _returnvalue_pitch _returnvalue_yaw) (`KismetMathLibrary.BreakRotator` (`SceneComponent.K2_GetComponentRotation` (`self.kartMesh`))))
  (`SceneComponent.K2_SetWorldRotation` (`self.kartMesh`) (`KismetMathLibrary.MakeRotator` _returnvalue_roll _returnvalue_pitch (+ _returnvalue_yaw (* (`self.steerValue`) (`self.steerMax`) delta))) false false))

(fn `UserConstructionScript`)